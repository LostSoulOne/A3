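; Anim notify that plays a unit sound effect during an animation, but only when the player is close enough.
; On notify, it compares the distance between the mesh component and player pawn 0 against the Distance variable.
; Within range, it plays Sound at the owning actor's location, scaled by Volume and with that actor as the sound's owner.
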(fn ReceivedNotify
  (params (MeshComp :type Skeletal%20Mesh%20Component%20Object%20Reference) (Animation :type Anim%20Sequence%20Base%20Object%20Reference))
  (bind _returnvalue (Transformation|GetWorldLocation MeshComp))
  (bind _returnvalue_2 (Game|Player|GetPlayerPawn 0))
  (bind _returnvalue_3 (Components|GetOwner MeshComp))
  (bind _distance (Variables|Default|GetDistance))
  (bind _rootcomponent (Variables|/Script/Engine.Actor|GetRootComponent _returnvalue_2))
  (bind _returnvalue_4 (Transformation|GetWorldLocation _rootcomponent))
  (bind _returnvalue_5 (Math|Vector|Distance(Vector) _returnvalue _returnvalue_4))
  (bind _returnvalue_6 (<= _returnvalue_5 _distance))
  (if _returnvalue_6
    (Audio|PlaySoundatLocation (Variables|Default|GetSound) (Transformation|GetWorldLocation (Variables|/Script/Engine.Actor|GetRootComponent _returnvalue_3)) "0, 0, 0" (Variables|Default|GetVolume) 1.0 0.0 0 0 _returnvalue_3)
    (else
      (return _returnvalue_6))))