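; Anim notify that shakes the local player's camera when an animation reaches it near the player.
; It compares the animated mesh's world location with the player 0 pawn's root location against a Distance threshold.
; Within range, it starts the configured Shake at a fixed Scale on player controller 0, with no falloff, and returns the range check result.
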(fn ReceivedNotify
  (params (MeshComp :type Skeletal%20Mesh%20Component%20Object%20Reference) (Animation :type Anim%20Sequence%20Base%20Object%20Reference))
  (bind _returnvalue (Transformation|GetWorldLocation MeshComp))
  (bind _returnvalue_2 (Game|Player|GetPlayerPawn 0))
  (bind _distance (Variables|Default|GetDistance))
  (bind _rootcomponent (Variables|/Script/Engine.Actor|GetRootComponent _returnvalue_2))
  (bind _returnvalue_3 (Transformation|GetWorldLocation _rootcomponent))
  (bind _returnvalue_4 (Math|Vector|Distance(Vector) _returnvalue _returnvalue_3))
  (bind _returnvalue_5 (<= _returnvalue_4 _distance))
  (if _returnvalue_5
    (Game|Feedback|ClientStartCameraShake (Game|GetPlayerController 0) (Variables|Default|GetShake) (Variables|Default|GetScale) "CameraLocal" "0, 0, 0"))
  (return _returnvalue_5))