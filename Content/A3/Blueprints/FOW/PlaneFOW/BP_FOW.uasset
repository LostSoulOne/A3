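; BP_FOW is a fog-of-war actor that reveals areas around RTS_UnitMonster_BP units by drawing into two render targets.
; Each tick it finds every unit, line-traces vertically onto the fog to get its hit UV, and draws a subtraction material sized by scan range.
; The secondary fog resets every tick to show current vision, while the main black fog accumulates cleared areas, cut only by moving units.
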(event Custom|SubstarctFromFog
  (params (VectorConversions :type Vector%202D%20Structure) (Value :type Float%20%28single-precision%29) (MainFog :type Boolean))
  ;[0.5417 0.5417 0.5417] Задаем вырезалке её координаты и размеры а затем вырезаем её из подложки
  (Rendering|Material|SetVectorParameterValue (Variables|Default|GetFogSubstraction) "DrawLocation" (Math|Conversions|ToLinearColor(Vector) (Math|Conversions|ToVector(Vector2D) VectorConversions)) :!class /Script/Engine.MaterialInstanceDynamic)
  (Rendering|Material|SetScalarParameterValue (Variables|Default|GetFogSubstraction) "DrawSize" Value :!class /Script/Engine.MaterialInstanceDynamic)
  (if MainFog
    (Rendering|DrawMaterialtoRenderTarget "/Game/A3/Blueprints/FOW/CorrectFog/T_FOW_RT.T_FOW_RT" (Variables|Default|GetFogSubstraction)))
  (Rendering|DrawMaterialtoRenderTarget "/Game/A3/Blueprints/FOW/CorrectFog/T_FOWsub_RT.T_FOWsub_RT" (Variables|Default|GetFogSubstraction)))

(event EventBeginPlay
  ;[0.5052 0.5052 0.5052] Создаем и задаем вырезалку а затем очищаем подложку
  (bind _returnvalue (Rendering|Material|CreateDynamicMaterialInstance "/Game/A3/Blueprints/FOW/CorrectFog/CorrcetFow_Substractor_M.CorrcetFow_Substractor_M" "None" :!class /Script/Engine.KismetMaterialLibrary))
  (Variables|Default|SetFogSubstraction _returnvalue)
  (Rendering|ClearRenderTarget2D "/Game/A3/Blueprints/FOW/CorrectFog/T_FOW_RT.T_FOW_RT")
  (Rendering|ClearRenderTarget2D "/Game/A3/Blueprints/FOW/CorrectFog/T_FOWsub_RT.T_FOWsub_RT" (Variables|Default|GetSubfogColor)))

(event EventTick
  (params (DeltaSeconds :type Float%20%28single-precision%29))
  ;[0.5365 0.5365 0.5365] Все монстры и их подклассы передают инфу о размерах круга обзора блюпринту тумана
  (Rendering|ClearRenderTarget2D "/Game/A3/Blueprints/FOW/CorrectFog/T_FOWsub_RT.T_FOWsub_RT" (Variables|Default|GetSubfogColor))
  (bind _outactors (Actor|GetAllActorsOfClass "/Game/A3/Blueprints/Units/MastersBP/RTS_UnitMonster_BP.RTS_UnitMonster_BP_C"))
  (for _array_element _outactors
    (Utilities|IsValid _array_element
      (:Is%20Valid
        (bind _asrts_unit_monster_bp (Utilities|Casting|CastToRTS_UnitMonster_BP _array_element))
        (bind _returnvalue (Physics|GetPhysicsLinearVelocity (Variables|/Script/Engine.Character|GetCapsuleComponent _asrts_unit_monster_bp) "None"))
        (bind (_fow_bp _textureuv _scanrange) (Utilities|GetUnitPosinFow _asrts_unit_monster_bp))
        ;;[0.5365 0.5365 0.5365] Тут чистим чёрный туман и нужно чтобы обычный тоже рисовался
        (CallFunction|SubstarctfromFog _fow_bp _textureuv _scanrange (> (Math|Vector|VectorLength _returnvalue) 5.0))))))

(fn ConstructionScript)