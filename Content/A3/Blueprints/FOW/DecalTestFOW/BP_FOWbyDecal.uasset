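; Fog of war test actor that carves revealed areas out of a fog render target on request.
; BeginPlay creates a dynamic instance of a subtractor material and clears the render target to opaque black.
; SubstarctFromFog feeds a 2D draw location and size into that material, then draws it onto the render target.
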(event Custom|SubstarctFromFog
  (params (VectorConversions :type Vector%202D%20Structure) (Value :type Float%20%28single-precision%29))
  (Rendering|Material|SetVectorParameterValue (Variables|Default|GetFogSubstraction) "DrawLocation" (Math|Conversions|ToLinearColor(Vector) (Math|Conversions|ToVector(Vector2D) VectorConversions)) :!class /Script/Engine.MaterialInstanceDynamic)
  (Rendering|Material|SetScalarParameterValue (Variables|Default|GetFogSubstraction) "DrawSize" Value :!class /Script/Engine.MaterialInstanceDynamic)
  (Rendering|DrawMaterialtoRenderTarget "/Game/A3/Blueprints/FOW/CorrectFog/T_FOW_RT.T_FOW_RT" (Variables|Default|GetFogSubstraction)))

(event EventBeginPlay
  (bind _returnvalue (Rendering|Material|CreateDynamicMaterialInstance "/Game/A3/Blueprints/FOW/CorrectFog/CorrcetFow_Substractor_M.CorrcetFow_Substractor_M" "None" :!class /Script/Engine.KismetMaterialLibrary))
  (Variables|Default|SetFogSubstraction _returnvalue)
  (Rendering|ClearRenderTarget2D "/Game/A3/Blueprints/FOW/CorrectFog/T_FOW_RT.T_FOW_RT"))

(fn ConstructionScript)