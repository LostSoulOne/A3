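; Fog-of-war actor for the RTS, with a plane scaled to the world size, that reveals what living Player-team monsters can see.
; Each tick it checks whether any unit moved, then line-traces a fan around each to its scan range so obstacles block vision.
; The hits become a triangle fan drawn into a canvas render target, cleared on each update.
; A material then draws onto the fog render target, which is cleared only at BeginPlay.
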(event EventBeginPlay
  ;[0.5052 0.5052 0.5052] Создаем и задаем вырезалку а затем очищаем подложку
  (bind _returnvalue (Rendering|Material|CreateDynamicMaterialInstance "/Game/A3/Blueprints/FOW/Vafog/LostVaFogMat.LostVaFogMat" "None" "None" :!class /Script/Engine.KismetMaterialLibrary))
  (Variables|Default|SetWhiteFog _returnvalue)
  (bind _returnvalue_2 (Rendering|Material|CreateDynamicMaterialInstance "/Game/A3/Blueprints/FOW/CorrectFog/T_FOWCanvas_RT_Mat.T_FOWCanvas_RT_Mat" "None" "None" :!class /Script/Engine.KismetMaterialLibrary))
  (Variables|Default|SetFogSubstraction _returnvalue_2)
  (Rendering|ClearRenderTarget2D "/Game/A3/Blueprints/FOW/CorrectFog/T_FOW_RT.T_FOW_RT")
  (Rendering|ClearRenderTarget2D "/Game/A3/Blueprints/FOW/CorrectFog/T_FOWCanvas_RT.T_FOWCanvas_RT" (Variables|Default|GetSubfogColor))
  (bind _returnvalue_3 (Rendering|Material|GetScalarParameterValue "/Game/A3/Blueprints/FOW/CorrectFog/CorrectFOW_Matpars.CorrectFOW_Matpars" "WorldSize" :!class /Script/Engine.KismetMaterialLibrary))
  (Transformation|SetRelativeScale3D (Variables|Default|GetPlane) (Math|Vector|MakeVector _returnvalue_3 _returnvalue_3 1.0)))

(event EventTick
  (params (DeltaSeconds :type Float%20%28single-precision%29))
  (bind _ai_friendlyactors (Variables|Default|GetAI_FriendlyActors))
  ;[0.5365 0.5365 0.5365] Все монстры и их подклассы передают инфу о размерах круга обзора блюпринту тумана
  (Utilities|Array|Clear (Variables|Default|GetAI_FriendlyActors))
  (bind _outactors (Actor|GetAllActorsOfClass "/Game/A3/Blueprints/Units/MastersBP/RTS_UnitMonster_BP.RTS_UnitMonster_BP_C"))
  (for _array_element _outactors
    (if (and (Utilities|Enum|Equal(Enum) (Variables|/Game/A3/Blueprints/Units/MastersBP/RTS_UnitMaster_BP.RTS_UnitMaster_BP_C|GetAI_Team _array_element) "Player") (not (Variables|/Game/A3/Blueprints/Units/MastersBP/RTS_UnitMonster_BP.RTS_UnitMonster_BP_C|GetInDeath _array_element)))
      (Utilities|Array|Add (Variables|Default|GetAI_FriendlyActors) _array_element)))
  (for _array_element_2 _ai_friendlyactors
    (CallFunction|CheckFogforUpdate _array_element_2))
  (if (Variables|Default|GetFogNeedUpdate)
    (for _array_element_3 _ai_friendlyactors
      (Utilities|IsValid _array_element_3
        (:Is%20Valid
          (CallFunction|MakeTrace _array_element_3)
          (CallFunction|PrepareTrinaglesforCanvas _array_element_3))))
    (Variables|Default|SetFogNeedUpdate false)
    (CallFunction|DrawFogTraceCanvas)
    (CallFunction|UpdateFogOLD)
    (Utilities|Array|Clear (Variables|Default|GetCanvasTriangles))))

(fn ConstructionScript)

(fn DrawFogTraceCanvas
  (Rendering|ClearRenderTarget2D "/Game/A3/Blueprints/FOW/CorrectFog/T_FOWCanvas_RT.T_FOWCanvas_RT" (Variables|Default|GetSubfogColor))
  (bind (_canvas _size _context) (Rendering|BeginDrawCanvastoRenderTarget "/Game/A3/Blueprints/FOW/CorrectFog/T_FOWCanvas_RT.T_FOWCanvas_RT"))
  (Class|Canvas|DrawTriangle _canvas 0 (Variables|Default|GetCanvasTriangles))
  (Rendering|EndDrawCanvastoRenderTarget _context)
  (return))

(fn UpdateFogOLD
  (params (Unit :type RTS%20Unit%20Monster%20BP%20Object%20Reference))
  (CallFunction|SubstractfromFog))

(fn CheckFogforUpdate
  (params (InputPin :type RTS%20Unit%20Master%20BP%20Object%20Reference))
  (bind _returnvalue (Transformation|GetActorLocation InputPin))
  (Utilities|IsValid InputPin
    (:Is%20Valid
      ;[1 1 1] Нужно убрать отсюда ичфрейм потом
      (if (Math|Vector|NotEqual(Vector) _returnvalue (Variables|/Game/A3/Blueprints/Units/MastersBP/RTS_UnitMaster_BP.RTS_UnitMaster_BP_C|GetLastFogPosition InputPin) 0.0001)
        (Variables|/Game/A3/Blueprints/Units/MastersBP/RTS_UnitMaster_BP.RTS_UnitMaster_BP_C|SetLastFogPosition InputPin _returnvalue)
        (Variables|Default|SetFogNeedUpdate true)))))

(fn SubstractfromFog
  (params (InVector2D :type Vector%202D%20Structure) (InputPin :type Float%20%28single-precision%29))
  (Rendering|DrawMaterialtoRenderTarget "/Game/A3/Blueprints/FOW/CorrectFog/T_FOW_RT.T_FOW_RT" (Variables|Default|GetFogSubstraction)))

(fn MakeTrace
  (params (Target :type RTS%20Unit%20Monster%20BP%20Object%20Reference))
  (bind _returnvalue (Transformation|GetActorLocation Target))
  (bind _baseeyeheight (Variables|/Script/Engine.Pawn|GetBaseEyeHeight Target))
  (bind _traceresults (Variables|Default|GetTraceResults))
  (bind _returnvalue_2 (+ (.z _returnvalue) _baseeyeheight))
  (bind _returnvalue_3 (Math|Vector|MakeVector (.x _returnvalue) (.y _returnvalue) _returnvalue_2))
  (Utilities|Array|Clear (Variables|Default|GetTraceResults))
  (for _index (range 0 (Variables|Default|GetNumTraces))
    (Rendering|Material|GetScalarParameterValue "/Game/A3/Blueprints/FOW/CorrectFog/CorrectFOW_Matpars.CorrectFOW_Matpars" "WorldSize" :!class /Script/Engine.KismetMaterialLibrary)
    (bind (_outhit _returnvalue_4) (Collision|LineTraceByChannel _returnvalue_3 (+ (* (Math|Vector|RotateVector (Math|Vector|RotateVector (Transformation|GetActorForwardVector Target) (Math|Rotator|MakeRotator 0.0 0.0 (/ (* (Variables|Default|GetNumTraces) (Variables|Default|GetTraceDegrees)) -2.0))) (Math|Rotator|MakeRotator 0.0 0.0 (* _index (Variables|Default|GetTraceDegrees)))) (* (Variables|/Game/A3/Blueprints/Units/MastersBP/RTS_UnitMonster_BP.RTS_UnitMonster_BP_C|GetUnitParScanrange Target) 2e+02)) _returnvalue_3) "TraceTypeQuery1" false 0 "None"))
    (if _returnvalue_4
      (Utilities|Array|Add _traceresults (+ (* (Math|Vector|RotateVector (Math|Vector|RotateVector (Transformation|GetActorForwardVector Target) (Math|Rotator|MakeRotator 0.0 0.0 (/ (* (Variables|Default|GetNumTraces) (Variables|Default|GetTraceDegrees)) -2.0))) (Math|Rotator|MakeRotator 0.0 0.0 (* _index (Variables|Default|GetTraceDegrees)))) 3e+01) (.Location (Collision|BreakHitResult _outhit))))
      (else
        (Utilities|Array|Add _traceresults (+ (* (Math|Vector|RotateVector (Math|Vector|RotateVector (Transformation|GetActorForwardVector Target) (Math|Rotator|MakeRotator 0.0 0.0 (/ (* (Variables|Default|GetNumTraces) (Variables|Default|GetTraceDegrees)) -2.0))) (Math|Rotator|MakeRotator 0.0 0.0 (* _index (Variables|Default|GetTraceDegrees)))) 3e+01) (+ (* (Math|Vector|RotateVector (Math|Vector|RotateVector (Transformation|GetActorForwardVector Target) (Math|Rotator|MakeRotator 0.0 0.0 (/ (* (Variables|Default|GetNumTraces) (Variables|Default|GetTraceDegrees)) -2.0))) (Math|Rotator|MakeRotator 0.0 0.0 (* _index (Variables|Default|GetTraceDegrees)))) (* (Variables|/Game/A3/Blueprints/Units/MastersBP/RTS_UnitMonster_BP.RTS_UnitMonster_BP_C|GetUnitParScanrange Target) 2e+02)) _returnvalue_3))))))
  (return))

(fn PrepareTrinaglesforCanvas
  (params (Unit :type RTS%20Unit%20Monster%20BP%20Object%20Reference))
  (bind _traceresults (Variables|Default|GetTraceResults))
  (for _index (range 0 (- (Utilities|Array|Length (Variables|Default|GetTraceResults)) 2))
    (bind _returnvalue (Rendering|Material|GetScalarParameterValue "/Game/A3/Blueprints/FOW/CorrectFog/CorrectFOW_Matpars.CorrectFOW_Matpars" "WorldSize" :!class /Script/Engine.KismetMaterialLibrary))
    (Utilities|Array|Add (Variables|Default|GetCanvasTriangles) (Utilities|Struct|MakeCanvasUVTri (Math|Conversions|ToVector2D(Vector) (Math|Vector|MakeVector (+ (.x (* (* (/ (Transformation|GetActorLocation Unit) (/ _returnvalue 1e+01)) -1.0) 1.0)) 5e+02) (+ (.y (* (* (/ (Transformation|GetActorLocation Unit) (/ _returnvalue 1e+01)) -1.0) 1.0)) 5e+02) 0.0)) "(X=0.000000,Y=0.000000)" "(R=1.000000,G=1.000000,B=1.000000,A=1.000000)" (Math|Conversions|ToVector2D(Vector) (+ (+ (/ (* (Utilities|Array|Get(acopy) _traceresults _index) -1.0) (* (/ _returnvalue 1e+02) 1e+01)) 5e+02) "0, 0, 0")) "(X=0.000000,Y=0.000000)" "(R=1.000000,G=1.000000,B=1.000000,A=1.000000)" (Math|Conversions|ToVector2D(Vector) (+ (+ (/ (* (Utilities|Array|Get(acopy) _traceresults (+ _index 1)) -1.0) (* (/ _returnvalue 1e+02) 1e+01)) 5e+02) "0, 0, 0")) "(X=0.000000,Y=0.000000)" "(R=1.000000,G=1.000000,B=1.000000,A=0.995000)")))
  (return))