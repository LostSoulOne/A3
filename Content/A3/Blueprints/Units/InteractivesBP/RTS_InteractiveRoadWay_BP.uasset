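; RTS interactive roadway actor that opens a map event on the player's HUD when an actor overlaps it.
; On overlap it passes its Event row name to the cached RTS player controller, with IsTalk blocking repeats until any overlap ends.
; The overlap does not filter by actor type; Tick's hero capsule check leads to no action.
; A map-parameter table lookup for setting Event sits unconnected in the construction script.
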(event EventBeginPlay
  (|CallParentFunction)
  (bind _asrts_player_controller_bp (Utilities|Casting|CastToRTS_PlayerController_BP (Game|GetPlayerController 0)))
  (Variables|Default|SetPlayerControllerRef _asrts_player_controller_bp))

(event Collision|EventActorBeginOverlap
  (params (OtherActor :type Actor%20Object%20Reference))
  (|CallParentFunction OtherActor)
  (if (not (Variables|Default|GetIsTalk))
    (Default|HUDOpenMapEvent (Variables|Default|GetPlayerControllerRef) (.rowname (Variables|Editor|GetEvent)))
    (Variables|Default|SetIsTalk true)))

(event EventTick
  (params (DeltaSeconds :type Float%20%28single-precision%29))
  (|CallParentFunction DeltaSeconds)
  (Utilities|IsValid (Utilities|Array|Get(acopy) (Collision|GetOverlappingActors (Variables|Default|GetCapsuleComponent) "/Game/A3/Blueprints/Units/MastersBP/RTS_UnitHero_BP.RTS_UnitHero_BP_C" :!class /Script/Engine.PrimitiveComponent))))

(event Collision|EventActorEndOverlap
  (params (OtherActor :type Actor%20Object%20Reference))
  (Variables|Default|SetIsTalk false))

(fn ConstructionScript
  (|CallParentFunction))