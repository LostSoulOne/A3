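; Master Blueprint for RTS building units, which takes its base stats from a data table.
; The construction script runs the parent's script, then looks up RowName in the DBaseBuildings table.
; A found row is stored in DTBuildings and supplies the unit's name and max health, converted to float.
; The event graph holds only disabled placeholder events, so this Blueprint adds no runtime logic.
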(event EventBeginPlay
  (|CallParentFunction) ; This node is disabled and will not be called.\nDrag off pins to build functionality.
)

(event Collision|EventActorBeginOverlap
  (params (OtherActor :type Actor%20Object%20Reference))
  (|CallParentFunction OtherActor) ; This node is disabled and will not be called.\nDrag off pins to build functionality.
)

(event EventTick
  (params (DeltaSeconds :type Float%20%28single-precision%29))
  (|CallParentFunction DeltaSeconds) ; This node is disabled and will not be called.\nDrag off pins to build functionality.
)

(fn ConstructionScript
  (|CallParentFunction)
  (bind _returnvalue (Utilities|GetDataTableRow "/Game/A3/DataFiles/dBaseBuildings.dBaseBuildings" (Variables|Default|GetRow%20Name))
    (:then
      (Variables|Default|SetDTBuildings _returnvalue)
      (Variables|Default|SetUnitMaxHealth (Math|Conversions|ToFloat(Integer) (.healthmax (Variables|Default|GetDTBuildings))))
      (Variables|Default|SetUnitName (.name (Variables|Default|GetDTBuildings))))))