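; AI controller for RTS monster units that handles move orders and draws path decals for selected units.
; Move orders project the destination onto the navmesh and restart AI MoveTo.
; On Tick, it offsets the cursor position into a two-column grid by selection index for the path target.
; When stationary or redirected, it rebuilds the navigation path on the unit's spline and spawns evenly spaced decals, shown while moving.
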(event Custom|EventMoveToLocOrAct
  (params (GoalLocation :type Vector))
  (AI|Navigation|StopMovement)
  (AI|AIMoveTo self GoalLocation 0 -1.0 "Enable" "Disable" true false false "Enable"))

(event Custom|EventSpawnDelay
  (params (Duration :type Float%20%28single-precision%29))
  (Utilities|FlowControl|Delay Duration))

(event EventBeginPlay)

(event EventTick
  (params (DeltaSeconds :type Float%20%28single-precision%29))
  (bind _ai_controlledpawnref (Variables|Default|GetAI_ControlledPawnRef))
  (Utilities|IsValid _ai_controlledpawnref
    (:Is%20Valid
      (if (Variables|/Game/A3/Blueprints/Units/MastersBP/RTS_UnitMaster_BP.RTS_UnitMaster_BP_C|GetUnitSelected _ai_controlledpawnref)
        (CallFunction|AIUnitSetupPathLocations)))))

(fn ConstructionScript)

(fn AIMovetoLocationC
  (params (MovePointLocation :type Vector))
  (CallFunction|AISetControlledPawnRef)
  (Variables|Default|SetMovePointLocation MovePointLocation)
  ;[1 1 1] Пока не использовал
  (Variables|/Game/A3/Blueprints/Units/MastersBP/RTS_UnitMonster_BP.RTS_UnitMonster_BP_C|SetLastMovementLocation (Variables|Default|GetAI_ControlledPawnRef) (Variables|Default|GetMovePointLocation))
  (Variables|Default|SetChangeDirection true)
  (CallFunction|EventMovetoLocorAct (.ProjectedLocation (AI|Navigation|ProjectPointtoNavigation (Variables|Default|GetMovePointLocation) 0 0 "0, 0, 0"))))

(fn AIUnitSetupPathLocations
  (bind _returnvalue (Game|Player|GetPlayerPawn 0))
  (Utilities|IsValid (Variables|Default|GetAI_ControlledPawnRef)
    (:Is%20Valid
      (bind _asrts_camera_pawn_bp (Utilities|Casting|CastToRTS_CameraPawn_BP _returnvalue))
      (bind _asrts_player_controller_bp (Utilities|Casting|CastToRTS_PlayerController_BP (Pawn|GetController _returnvalue)))
      (for (_array_element _array_index) (Variables|/Game/A3/Blueprints/Player/RTS_PlayerController_BP.RTS_PlayerController_BP_C|GetSelected%20Characters _asrts_player_controller_bp)
        (bind _asrts_unit_monster_bp (Utilities|Casting|CastToRTS_UnitMonster_BP _array_element))
        (if (== _asrts_unit_monster_bp (Variables|Default|GetAI_ControlledPawnRef))
          (CallFunction|AIUnitShowPath (+ (Math|Vector|MakeVector (* (/ _array_index 2) 2e+02) (* (Math|Integer|%(Integer) _array_index 2) 2e+02) 0.0) (Transformation|GetWorldLocation (Variables|/Game/A3/Blueprints/Player/RTS_CameraPawn_BP.RTS_CameraPawn_BP_C|GetCursorToWorld _asrts_camera_pawn_bp)))))))))

(fn AIUnitShowPath
  (params (TargetPosition :type Vector%20%28by%20ref%29))
  (bind _locationdecals (Variables|Default|GetLocationDecals))
  (bind _ai_controlledpawnref (Variables|Default|GetAI_ControlledPawnRef))
  (CallFunction|AISetControlledPawnRef)
  (if (Variables|/Game/A3/Blueprints/Units/MastersBP/RTS_UnitMaster_BP.RTS_UnitMaster_BP_C|GetUnitSelected (Variables|Default|GetAI_ControlledPawnRef))
    (if (or (Math|Vector|Equal(Vector) (Pawn|Components|CharacterMovement|GetLastUpdateVelocity (Variables|/Script/Engine.Character|GetCharacterMovement (Variables|Default|GetAI_ControlledPawnRef))) "0, 0, 0" 2.0) (Variables|Default|GetChangeDirection))
      (for _array_element _locationdecals
        (Utilities|IsValid _array_element
          (:Is%20Valid
            (Rendering|SetVisibility _array_element false false))))
      (Utilities|Array|Clear (Variables|Default|GetUnit_PathPoints))
      ;[1 1 1] Если дали новую команду
      (Variables|Default|SetChangeDirection false)
      (Variables|Default|SetPrevTargetLocation TargetPosition)
      (bind _returnvalue (Class|NavigationSystemV1|FindPathtoLocationSynchronously (Transformation|GetActorLocation _ai_controlledpawnref) TargetPosition _ai_controlledpawnref 0))
      (Spline|ClearSplinePoints (Variables|/Game/A3/Blueprints/Units/MastersBP/RTS_UnitMonster_BP.RTS_UnitMonster_BP_C|GetSpline (Variables|Default|GetAI_ControlledPawnRef)) true)
      (for _array_element_2 (Variables|/Script/NavigationSystem.NavigationPath|GetPathPoints _returnvalue)
        (Spline|AddSplinePoint (Variables|/Game/A3/Blueprints/Units/MastersBP/RTS_UnitMonster_BP.RTS_UnitMonster_BP_C|GetSpline (Variables|Default|GetAI_ControlledPawnRef)) (+ _array_element_2 "0, 0,30.000000") "World" true))
      (bind _index (Utilities|FlowControl|ForLoopwithBreak 0 (.ReturnValue (Math|Float|Division(WholeandRemainder) (Spline|GetSplineLength (Variables|/Game/A3/Blueprints/Units/MastersBP/RTS_UnitMonster_BP.RTS_UnitMonster_BP_C|GetSpline (Variables|Default|GetAI_ControlledPawnRef))) (Variables|Default|GetUnit_PathPointsSpacing))))
        (:LoopBody
          (Utilities|Array|Add (Variables|Default|GetUnit_PathPoints) (+ (Spline|GetLocationatDistanceAlongSpline (Variables|/Game/A3/Blueprints/Units/MastersBP/RTS_UnitMonster_BP.RTS_UnitMonster_BP_C|GetSpline (Variables|Default|GetAI_ControlledPawnRef)) (* _index (Variables|Default|GetUnit_PathPointsSpacing)) "World") "0, 0, 0")))
        (:Completed
          (CallFunction|AISpawnMovePoints (Variables|Default|GetUnit_PathPoints) "100.000000,24.000000,24.000000" "/Game/A3/Textures/UI/CursorTest/M_SelectionMovement_Decal_Inst.M_SelectionMovement_Decal_Inst" 1.0)))
      (else
        (for _array_element_3 _locationdecals
          (Utilities|IsValid _array_element_3
            (:Is%20Valid
              (Rendering|SetVisibility _array_element_3 true false))))))))

(fn AISetControlledPawnRef
  (bind _asrts_unit_monster_bp (Utilities|Casting|CastToRTS_UnitMonster_BP (Pawn|GetControlledPawn)))
  (Variables|Default|SetAI_ControlledPawnRef _asrts_unit_monster_bp)
  (return))

(fn AISpawnMovePoints
  (params (PointsVectors :type Array%20of%20Vectors) (DecalSize :type Vector) (DecalMat :type Material%20Interface%20Object%20Reference) (LifeSpan :type Float%20%28single-precision%29))
  (bind _ai_controlledpawnref (Variables|Default|GetAI_ControlledPawnRef))
  (bind _ai_controlledpawnref_2 (Variables|Default|GetAI_ControlledPawnRef))
  (bind _changedirection (Variables|Default|GetChangeDirection))
  (bind _locationdecals (Variables|Default|GetLocationDecals))
  (bind _selectround (Variables|/Game/A3/Blueprints/Units/MastersBP/RTS_UnitMaster_BP.RTS_UnitMaster_BP_C|GetSelectRound _ai_controlledpawnref))
  (bind _charactermovement (Variables|/Script/Engine.Character|GetCharacterMovement _ai_controlledpawnref_2))
  (bind _returnvalue (Pawn|Components|CharacterMovement|GetLastUpdateVelocity _charactermovement))
  (bind _relativescale3d (Variables|/Script/Engine.SceneComponent|GetRelativeScale3D _selectround))
  (bind _returnvalue_2 (Math|Vector|Equal(Vector) _returnvalue "0, 0, 0" 2.0))
  (bind _returnvalue_3 (or _returnvalue_2 _changedirection))
  (CallFunction|AISetControlledPawnRef)
  (for _array_element (Variables|Default|GetLocationDecals)
    (Utilities|IsValid _array_element
      (:Is%20Valid
        (Components|DestroyComponent _array_element))))
  (Utilities|Array|Clear (Variables|Default|GetLocationDecals))
  (for (_array_element_2 _array_index) PointsVectors
    (if (== _array_index (- (Utilities|Array|Length PointsVectors) 1))
      (bind _returnvalue_4 (Rendering|Decal|SpawnDecalatLocation "/Game/A3/Textures/UI/CursorTest/M_SelectionMovementTarget_D.M_SelectionMovementTarget_D" (Math|Vector|MakeVector 128.0 (* (.y (Variables|/Script/Engine.DecalComponent|GetDecalSize _selectround)) (.y _relativescale3d) 1.4) (* (.z (Variables|/Script/Engine.DecalComponent|GetDecalSize _selectround)) (.z _relativescale3d) 1.4)) _array_element_2 "-90.000000,0.000000,0.000000" 5.0))
      (Utilities|Array|Add _locationdecals _returnvalue_4)
      (if _returnvalue_3
        (Rendering|SetVisibility _returnvalue_4 false false)
        (else
          (Rendering|SetVisibility _returnvalue_4 true false)))
      (else
        (bind _returnvalue_5 (Rendering|Decal|SpawnDecalatLocation DecalMat DecalSize _array_element_2 "-90.000000,0.000000,0.000000" LifeSpan))
        (Utilities|Array|Add _locationdecals _returnvalue_5)
        (if _returnvalue_3
          (Rendering|SetVisibility _returnvalue_5 false false)
          (else
            (Rendering|SetVisibility _returnvalue_5 true false))))))
  (return))