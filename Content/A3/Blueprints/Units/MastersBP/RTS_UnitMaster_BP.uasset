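; Base RTS unit with health bar, selection feedback, AI movement and item inventory.
; BeginPlay fits the health bar and selection ring to the capsule and caches the unit controller.
; Selection and focus drive ring visibility, bar opacity and a custom-depth hover highlight, while move orders use navmesh-projected AI MoveTo with a replaceable destination decal.
; Pickups stack non-magic items by row name and keep magic ones separate; item removal is an empty stub.
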(event EventTick
  (params (DeltaSeconds :type Float%20%28single-precision%29)))

(event Collision|EventActorBeginOverlap
  (params (OtherActor :type Actor%20Object%20Reference)))

(event EventBeginPlay
  (bind _capsulecomponent (Variables|Collision|GetCapsuleComponent))
  (bind _capsulecomponent_2 (Variables|Collision|GetCapsuleComponent))
  (bind _returnvalue (Components|Capsule|GetScaledCapsuleRadius _capsulecomponent))
  (bind _capsulehalfheight (Variables|/Script/Engine.CapsuleComponent|GetCapsuleHalfHeight _capsulecomponent_2))
  (bind _returnvalue_2 (/ _returnvalue 42.0))
  ;[1 1 1] Хелсбар
  (bind _asai_health_bar (Utilities|Casting|CastToAI_HealthBar (UserInterface|GetUserWidgetObject (Variables|Components|GetHealthBar))))
  (Variables|/Game/A3/Widgets/AI_HealthBar.AI_HealthBar_C|SetHealthBarOwner _asai_health_bar self)
  (Variables|/Game/A3/Widgets/AI_HealthBar.AI_HealthBar_C|SetHBWide _asai_health_bar (+ (Components|Capsule|GetScaledCapsuleRadius _capsulecomponent_2) 4e+01))
  (Transformation|SetRelativeLocation (Variables|Components|GetHealthBar) (Math|Vector|MakeVector 0.0 0.0 _capsulehalfheight) false false)
  (Variables|Default|SetBaseEyeHeight _capsulehalfheight)
  (Transformation|SetRelativeLocation (Variables|Components|GetSelectRound) (Math|Vector|MakeVector 0.0 0.0 (+ (* (Variables|/Script/Engine.CapsuleComponent|GetCapsuleHalfHeight (Variables|Collision|GetCapsuleComponent)) -1.0) 5.0)) false false)
  (Transformation|SetRelativeScale3D (Variables|Components|GetSelectRound) (Math|Vector|MakeVector _returnvalue_2 _returnvalue_2 _returnvalue_2))
  (bind _asrts_unit_controller_master_bp (Utilities|Casting|CastToRTS_Unit_Controller_Master_BP (Pawn|GetController)))
  (Variables|References|SetControllerRef _asrts_unit_controller_master_bp)
  (Variables|Navigation|SetStartRelativeLocation (Variables|/Script/Engine.SceneComponent|GetRelativeLocation (Variables|Character|GetMesh)))
  (Variables|Navigation|SetStartWorldLocation (Transformation|GetWorldLocation (Variables|Collision|GetCapsuleComponent))))

(fn ConstructionScript)

(fn AddItemtoInventory
  (params (TakenItem :type U%20Data%20Object%20Reference))
  (Game|ConstructObjectfromClass "/Game/A3/Blueprints/Inventory/UData.UData_C" self)
  (LocalVariables|SetTakenItemLocal TakenItem)
  (Variables|/Game/A3/Blueprints/Inventory/UData.UData_C|SetData (LocalVariables|GetTakenItemLocal) (Variables|/Game/A3/Blueprints/Inventory/UData.UData_C|GetData TakenItem))
  (Utilities|FlowControl|Sequence
    (:then_0
      (LocalVariables|SetTakenItemRowNameLocal (.rowitemname (Variables|/Game/A3/Blueprints/Inventory/UData.UData_C|GetData (LocalVariables|GetTakenItemLocal))))
      (bind _output_get (LocalVariables|SetTakenItemCountLocal (.count (Variables|/Game/A3/Blueprints/Inventory/UData.UData_C|GetData (LocalVariables|GetTakenItemLocal)))))
      (LocalVariables|SetIsMagicLocal (!= (Utilities|Map|Length (.magicparameters (Variables|/Game/A3/Blueprints/Inventory/UData.UData_C|GetData (LocalVariables|GetTakenItemLocal)))) 0))
      (bind _outtext (CallFunction|LSGetTextfromStringTable (LocalVariables|GetTakenItemRowNameLocal)))
      (if (== (Variables|MasterParams|GetUnitClass) 5)
        (if (Utilities|Enum|Equal(Enum) (LocalVariables|GetTakenItemRowNameLocal) "rem1")
          (Development|PrintString (Utilities|String|Append (Utilities|String|Append "Вы подобрали: " (Utilities|String|ToString(Text) _outtext)) ":  " (Utilities|String|ToString(Integer) (LocalVariables|GetTakenItemCountLocal))) true true "(R=0.376262,G=0.191202,B=0.030714,A=1.000000)" 1e+01)
          (else
            (Development|PrintString (Utilities|String|Append "Вы подобрали: " (Utilities|String|ToString(Text) _outtext)) true true "(R=0.376262,G=0.191202,B=0.030714,A=1.000000)" 1e+01)))))
    (:then_1
      (if (LocalVariables|GetIsMagicLocal)
        (Utilities|Array|Add (Variables|System|GetInventoryItemsUData) (LocalVariables|GetTakenItemLocal) :!label _label)
        (else
          (for _array_element (Variables|System|GetInventoryItemsUData)
            (bind _output_get_2 (LocalVariables|SetDataLocal (Variables|/Game/A3/Blueprints/Inventory/UData.UData_C|GetData _array_element)))
            (if (and (Utilities|Enum|Equal(Enum) (LocalVariables|GetTakenItemRowNameLocal) (.RowItemName (Utilities|Struct|BreakItemInfoData _output_get_2))) (== (Utilities|Map|Length (.MagicParameters (Utilities|Struct|BreakItemInfoData _output_get_2))) 0))
              (Utilities|Struct|SetmembersinItemInfoData (Variables|/Game/A3/Blueprints/Inventory/UData.UData_C|GetData _array_element) (+ (.Count (Utilities|Struct|BreakItemInfoData _output_get_2)) (LocalVariables|GetTakenItemCountLocal)))
              (LocalVariables|SetItemFound true)))
          (if (not (LocalVariables|GetItemFound))
            (goto _label)
            (else
              _))))
      (return (LocalVariables|GetTakenItemLocal)))))

(fn AICheckSelectionandFocus
  (bind _selectround (Variables|Components|GetSelectRound))
  (bind _selectround_2 (Variables|Components|GetSelectRound))
  (bind _selectround_3 (Variables|Components|GetSelectRound))
  (if (Variables|Selector|GetUnitFocused)
    (if (and (not (Variables|/Script/Engine.SceneComponent|GetbVisible _selectround_2)) (Variables|Selector|GetUnitSelected))
      (Rendering|SetVisibility _selectround_2 true false))
    (if (Variables|Selector|GetUnitSelected)
      (Rendering|SetRenderCustomDepth (Variables|Default|GetCylinderCollisionMesh) false)
      (bind _asai_health_bar (Utilities|Casting|CastToAI_HealthBar (UserInterface|GetWidget (Variables|Components|GetHealthBar))))
      (Default|SetHealthbarOpacity _asai_health_bar 1.0)
      (else
        (Rendering|SetRenderCustomDepth (Variables|Default|GetCylinderCollisionMesh) true)
        (bind _asai_health_bar_2 (Utilities|Casting|CastToAI_HealthBar (UserInterface|GetWidget (Variables|Components|GetHealthBar))))
        (Default|SetHealthbarOpacity _asai_health_bar_2 0.5)))
    (elif (Variables|Selector|GetUnitSelected)
      (if (Variables|/Script/Engine.SceneComponent|GetbVisible _selectround)
        _
        (else
          (Rendering|SetVisibility _selectround true false)))
      (Rendering|SetRenderCustomDepth (Variables|Default|GetCylinderCollisionMesh) false)
      (bind _asai_health_bar_3 (Utilities|Casting|CastToAI_HealthBar (UserInterface|GetWidget (Variables|Components|GetHealthBar))))
      (Default|SetHealthbarOpacity _asai_health_bar_3 1.0)
      (else
        (if (Variables|/Script/Engine.SceneComponent|GetbVisible _selectround_3)
          (Rendering|SetVisibility _selectround_3 false false))
        (Rendering|SetRenderCustomDepth (Variables|Default|GetCylinderCollisionMesh) false)
        (bind _asai_health_bar_4 (Utilities|Casting|CastToAI_HealthBar (UserInterface|GetWidget (Variables|Components|GetHealthBar))))
        (Default|SetHealthbarOpacity _asai_health_bar_4 0.5)))))

(fn AIUnitMovetoLocation
  (params (MovePointLocation :type Vector))
  (bind _output_get (Variables|Navigation|SetMovePointLocation MovePointLocation))
  (AI|Navigation|MovetoLocation (AI|GetAIController self) (.ProjectedLocation (AI|Navigation|ProjectPointtoNavigation _output_get 0 0 "0, 0, 0")) -1.0 true true false false 0)
  (Utilities|IsValid (Variables|Default|GetPreviousLocationDecal)
    (:Is%20Valid
      (Components|DestroyComponent (Variables|Default|GetPreviousLocationDecal)))
    (:Is%20Not%20Valid
      _))
  (bind _returnvalue (Rendering|Decal|SpawnDecalatLocation "/Game/A3/Textures/UI/CursorTest/M_SelectionGood_Decal.M_SelectionGood_Decal" "32.000000,32.000000,32.000000" _output_get "-90.000000,0.000000,0.000000" 0.0))
  (Variables|Default|SetPreviousLocationDecal _returnvalue))

(fn RemoveItemfromInventory
  (params (Dimension%201 :type Integer)))