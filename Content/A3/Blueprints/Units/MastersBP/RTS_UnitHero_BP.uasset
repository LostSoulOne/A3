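; RTS hero unit Blueprint handling melee combos and warrior or mage skill progression.
; Tick plays chained attack montages when AI is ready, buffering repeats through SaveAttack.
; Construction seeds main and secondary skills as experience; HeroTakeExperience maps damage type to skill, levels it on an exponential curve, then recalculates parameters and max HP/mana from strength, wisdom and total experience.
; Only Sword applies the reduced non-main experience rate.
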(event Custom|ResetCombo
  ;[1 1 1] Combo System Setup.
  (Variables|Default|SetAttackCount 0)
  (Variables|Default|SetSaveAttack false)
  (Variables|Default|SetIsAttacking false))

(event Custom|ComboAttackSave
  (bind _meleespeed (Variables|Default|GetMeleeSpeed))
  ;[1 1 1] Combo System Setup.
  (if (Variables|Default|GetSaveAttack)
    (Variables|Default|SetSaveAttack false)
    (switch int (Variables|Default|GetAttackCount)
      (:0
        (Variables|Default|SetAttackCount 1)
        (Animation|PlayAnimMontage "/Game/A3/Geometry/Units/TestGirl/AnimsGreystone/Attack_PrimaryA_Montage.Attack_PrimaryA_Montage" _meleespeed "None"))
      (:1
        (Variables|Default|SetAttackCount 2)
        (Animation|PlayAnimMontage "/Game/A3/Geometry/Units/TestGirl/AnimsGreystone/Attack_PrimaryB_Montage.Attack_PrimaryB_Montage" _meleespeed "None"))
      (:2
        (Variables|Default|SetAttackCount 0)
        (Animation|PlayAnimMontage "/Game/A3/Geometry/Units/TestGirl/AnimsGreystone/Attack_PrimaryC_Montage.Attack_PrimaryC_Montage" _meleespeed "None"))
      (:3
        (Variables|Default|SetAttackCount 4)
        (Animation|PlayAnimMontage "/Game/A3/Geometry/Units/TestGirl/AnimsGreystone/Attack_PrimaryD_Montage.Attack_PrimaryD_Montage" _meleespeed "None")))))

(event EventBeginPlay
  (|CallParentFunction)
  (CallFunction|CheckMaxHPMP)
  (Variables|Default|SetUnitHealth (Variables|Default|GetUnitMaxHealth)))

(event Collision|EventActorBeginOverlap
  (params (OtherActor :type Actor%20Object%20Reference))
  (|CallParentFunction OtherActor) ; This node is disabled and will not be called.\nDrag off pins to build functionality.
)

(event EventTick
  (params (DeltaSeconds :type Float%20%28single-precision%29))
  (|CallParentFunction DeltaSeconds)
  (if (and (Variables|Default|GetAI_ReadyToAttack) (not (Variables|Default|GetInDeath)))
    ;[1 1 1] Simple attack setup. Intentionally not using inputs so that this will "just work" with the 3rd Person Template. If you were doing this for real, you would set up a proper input.
    (Variables|Default|SetMeleeSpeed 1.4)
    ;[1 1 1] Combo System Setup.
    (if (Variables|Default|GetIsAttacking)
      (Variables|Default|SetSaveAttack true)
      (else
        (Variables|Default|SetIsAttacking true)
        (switch int (Variables|Default|GetAttackCount)
          (:0
            (Variables|Default|SetAttackCount 1)
            (Animation|PlayAnimMontage "/Game/A3/Geometry/Units/TestGirl/AnimsGreystone/Attack_PrimaryA_Montage.Attack_PrimaryA_Montage" (Variables|Default|GetMeleeSpeed) "None"))
          (:1
            (Variables|Default|SetAttackCount 2)
            (Animation|PlayAnimMontage "/Game/A3/Geometry/Units/TestGirl/AnimsGreystone/Attack_PrimaryB_Montage.Attack_PrimaryB_Montage" (Variables|Default|GetMeleeSpeed) "None"))
          (:2
            (Variables|Default|SetAttackCount 0)
            (Animation|PlayAnimMontage "/Game/A3/Geometry/Units/TestGirl/AnimsGreystone/Attack_PrimaryC_Montage.Attack_PrimaryC_Montage" (Variables|Default|GetMeleeSpeed) "None"))
          (:3
            (Variables|Default|SetAttackCount 4)
            (Animation|PlayAnimMontage "/Game/A3/Geometry/Units/TestGirl/AnimsGreystone/Attack_PrimaryD_Montage.Attack_PrimaryD_Montage" (Variables|Default|GetMeleeSpeed) "None")))))))

(event Input|MouseEvents|LeftMouseButton
  (params (Key :type Key%20Structure :default "None"))
  ;[1 1 1] Simple attack setup. Intentionally not using inputs so that this will "just work" with the 3rd Person Template. If you were doing this for real, you would set up a proper input.
)

(event Input|GamepadEvents|GamepadFaceButtonLeft
  (params (Key :type Key%20Structure :default "None"))
  ;[1 1 1] Simple attack setup. Intentionally not using inputs so that this will "just work" with the 3rd Person Template. If you were doing this for real, you would set up a proper input.
)

(fn ConstructionScript
  (|CallParentFunction)
  (CallFunction|HeroCalculateParameters)
  (CallFunction|HumanCalculateParameters))

(fn CheckMaxHeroPar
  (params (ClassMultiplier :type Float%20%28single-precision%29) (StreWis :type Integer))
  (bind _returnvalue (Math|Conversions|ToFloat(Integer) StreWis))
  (LocalVariables|SetClassMultiplierLocal ClassMultiplier)
  (return (+ (* (Math|Float|Truncate (/ (* (LocalVariables|GetClassMultiplierLocal) (Math|Float|Loge (+ (/ (Math|Conversions|ToFloat(Integer) (Variables|HeroParams|GetUnitParExperience)) 5e+03) 1.0))) (Math|Float|Loge 1.1))) (+ (/ (Math|Float|Power 1.1 (Math|Conversions|ToFloat(Integer) StreWis)) 1e+02) 1.0)) (+ (* (LocalVariables|GetClassMultiplierLocal) _returnvalue) (* (/ _returnvalue 5e+01) (Math|Float|Power 1.1 _returnvalue))))))

(fn CheckMaxHPMP
  (if (> (Variables|Default|GetUnitClass) 3)
    (if (== (Variables|Default|GetUnitSpecialization) 0)
      (bind _returnvalue (CallFunction|CheckMaxHeroPar 2.0 (Variables|Default|GetUnitParStrenght)))
      (Variables|Default|SetUnitMaxHealth _returnvalue)
      (Variables|Default|SetUnitParMaxMana 0)
      (else
        (bind _returnvalue_2 (CallFunction|CheckMaxHeroPar 2.0 (Variables|Default|GetUnitParStrenght)))
        (Variables|Default|SetUnitMaxHealth (/ _returnvalue_2 2.0))
        (bind _returnvalue_3 (CallFunction|CheckMaxHeroPar 2.0 (Variables|Default|GetUnitParWisdom)))
        (Variables|Default|SetUnitParMaxMana (Math|Float|Truncate _returnvalue_3))))
    (return)))

(fn HeroSetSkills
  (if (== (Variables|Default|GetUnitSpecialization) 0)
    ;[1 1 1] Это всё залупа, нужно давать опытом эти скилы в тихом режиме
    (Variables|Default|SetUnitSkillBow 10)
    (switch int (Variables|HeroParams|GetMainSkill)
      (:Default
        _)
      (:0
        _)
      (:1
        (Variables|Default|SetUnitSkillSword 20))
      (:2
        (Variables|Default|SetUnitSkillAxe 20))
      (:3
        (Variables|Default|SetUnitSkillMace 20))
      (:4
        (Variables|Default|SetUnitSkillSpear 20))
      (:5
        _))
    (else
      (Variables|Default|SetUnitSkillAstral 10)
      (switch int (Variables|HeroParams|GetMainSkill)
        (:Default
          _)
        (:0
          _)
        (:1
          (Variables|Default|SetUnitSkillFire 20))
        (:2
          (Variables|Default|SetUnitSkillWater 20))
        (:3
          (Variables|Default|SetUnitSkillAir 20))
        (:4
          (Variables|Default|SetUnitSkillEarth 20))
        (:5
          _))))
  (return))

(fn HeroCalculateParameters
  (bind _mainskill (Variables|HeroParams|GetMainSkill))
  (if (== (Variables|Default|GetUnitSpecialization) 0)
    (LocalVariables|SetMainLocal (Utilities|Enum|ByteToEnumDamageTypesEnum (Math|Conversions|ToByte(Integer) (+ _mainskill 1))))
    (LocalVariables|SetOtherLocal "NewEnumerator9")
    (else
      (LocalVariables|SetMainLocal (Utilities|Enum|ByteToEnumDamageTypesEnum (Math|Conversions|ToByte(Integer) (+ _mainskill 6))))
      (LocalVariables|SetOtherLocal "NewEnumerator4")))
  (bind _out (CallFunction|HeroA3Skill2Exp 2e+01))
  (CallFunction|HeroUpdateSkillsbyExp (LocalVariables|GetMainLocal) _out 0.0 true)
  (bind _out_2 (CallFunction|HeroA3Skill2Exp 1e+01))
  (CallFunction|HeroUpdateSkillsbyExp (LocalVariables|GetOtherLocal) _out_2 0.0 true)
  (return))

(fn UnitMakeMeleeDamage
  (|CallParentFunction))

(fn HeroTakeExperience
  (params (DamageType :type Damage%20Type%20Object%20Reference) (DamageCount :type Float%20%28single-precision%29) (MaxHP :type Float%20%28single-precision%29) (Killed :type Boolean) (EXP :type Float%20%28single-precision%29))
  (bind _returnvalue (Utilities|GetClass DamageType))
  (bind _unitparmind (Variables|Default|GetUnitParMind))
  (bind _returnvalue_2 (Math|Conversions|ToFloat(Integer) _unitparmind))
  (bind _returnvalue_3 (/ _returnvalue_2 6e+01))
  (bind _returnvalue_4 (+ 0.125 _returnvalue_3))
  (bind _returnvalue_5 (* EXP _returnvalue_4))
  (Utilities|FlowControl|Sequence
    (:then_1
      (if (== _returnvalue "/Game/A3/Blueprints/Interaction/Damage/DmgTypes_SwordBP.DmgTypes_SwordBP_C")
        (LocalVariables|SetDamageTypeLocal "NewEnumerator5")))
    (:then_2
      (if (== _returnvalue "/Game/A3/Blueprints/Interaction/Damage/DmgTypes_AxeBP.DmgTypes_AxeBP_C")
        (LocalVariables|SetDamageTypeLocal "NewEnumerator7")))
    (:then_3
      (if (== _returnvalue "/Game/A3/Blueprints/Interaction/Damage/DmgTypes_MaceBP.DmgTypes_MaceBP_C")
        (LocalVariables|SetDamageTypeLocal "NewEnumerator6")))
    (:then_4
      (if (== _returnvalue "/Game/A3/Blueprints/Interaction/Damage/DmgTypes_SpearBP.DmgTypes_SpearBP_C")
        (LocalVariables|SetDamageTypeLocal "NewEnumerator8")))
    (:then_5
      (if (== _returnvalue "/Game/A3/Blueprints/Interaction/Damage/DmgTypes_ArcheryBP.DmgTypes_ArcheryBP_C")
        (LocalVariables|SetDamageTypeLocal "NewEnumerator9")))
    (:then_6
      (if (== _returnvalue "/Game/A3/Blueprints/Interaction/Damage/DmgTypes_FireBP.DmgTypes_FireBP_C")
        (LocalVariables|SetDamageTypeLocal "NewEnumerator0")
        (Development|PrintString "Fire")))
    (:then_7
      (if (== _returnvalue "/Game/A3/Blueprints/Interaction/Damage/DmgTypes_WaterBP.DmgTypes_WaterBP_C")
        (LocalVariables|SetDamageTypeLocal "NewEnumerator1")))
    (:then_8
      (if (== _returnvalue "/Game/A3/Blueprints/Interaction/Damage/DmgTypes_WindBP.DmgTypes_WindBP_C")
        (LocalVariables|SetDamageTypeLocal "NewEnumerator2")))
    (:then_9
      (if (== _returnvalue "/Game/A3/Blueprints/Interaction/Damage/DmgTypes_EarthBP.DmgTypes_EarthBP_C")
        (LocalVariables|SetDamageTypeLocal "NewEnumerator3")))
    (:then_10
      (if (== _returnvalue "/Game/A3/Blueprints/Interaction/Damage/DmgTypes_AstralBP.DmgTypes_AstralBP_C")
        (LocalVariables|SetDamageTypeLocal "NewEnumerator4")))
    (:then_11
      (if (== _returnvalue "/Game/A3/Blueprints/Interaction/Damage/DmgTypes_MonsterBP.DmgTypes_MonsterBP_C")
        (LocalVariables|SetDamageTypeLocal "NewEnumerator11")))
    (:then_12
      (if (== _returnvalue "/Game/A3/Blueprints/Interaction/Damage/DmgTypes_IgnoreArmourBP.DmgTypes_IgnoreArmourBP_C")
        (LocalVariables|SetDamageTypeLocal "NewEnumerator12")))
    (:then_13
      (if Killed
        (LocalVariables|SetResultExpLocal _returnvalue_5)
        (else
          (LocalVariables|SetResultExpLocal (+ (* (Math|Float|SafeDivide DamageCount MaxHP) _returnvalue_5) 2.0))))
      (LocalVariables|SetResultExpNotMainLocal (+ (Math|Float|SafeDivide (- (LocalVariables|GetResultExpLocal) 2.0) 8.0) 1.0))
      (CallFunction|HeroUpdateSkillsbyExp (LocalVariables|GetDamageTypeLocal) (LocalVariables|GetResultExpLocal) (LocalVariables|GetResultExpNotMainLocal) false)
      (CallFunction|HumanCalculateParameters)
      (CallFunction|CheckMaxHPMP)
      (return))))

(fn HeroCalculateResultExp
  (params (ExpCur :type Float%20%28single-precision%29) (ExpLocal :type Float%20%28single-precision%29) (Skill :type Float%20%28single-precision%29) (NoClamp :type Boolean))
  (if (not NoClamp)
    (LocalVariables|SetResultLocal (+ ExpCur (Math|Float|Clamp(Float) ExpLocal 0.0 (* 2e+01 (Math|Float|Power 1.1 Skill)))))
    (else
      (LocalVariables|SetResultLocal (+ ExpCur ExpLocal))))
  (return (LocalVariables|GetResultLocal)))

(fn HeroA3Skill2Exp
  (params (Skill :type Float%20%28single-precision%29))
  (return (* 1e+03 (- (Math|Float|Power 1.1 Skill) 1.0))))

(fn HeroUpdateSkillsbyExp
  (params (Selection :type DamageTypesEnum%20Enum :default "NewEnumerator10") (ResultExp :type Float%20%28single-precision%29) (ResultExpNotMain :type Float%20%28single-precision%29) (NoClamp :type Boolean))
  (bind _unitspecialization (Variables|Default|GetUnitSpecialization))
  (bind _returnvalue (== _unitspecialization 1))
  (LocalVariables|SetNoClampLocal NoClamp)
  (LocalVariables|SetResultExpLocal ResultExp)
  (LocalVariables|SetResultExpNotMainLocal ResultExpNotMain)
  (Utilities|FlowControl|Sequence
    (:then_0
      (switch Utilities|FlowControl|Switch|SwitchonDamageTypesEnum Selection
        (:NewEnumerator5
          (if (== (Variables|HeroParams|GetMainSkill) 1)
            (bind _resultexp (CallFunction|HeroCalculateResultExp (Variables|HeroParams|GetUnitParExpSword) (LocalVariables|GetResultExpLocal) (Math|Conversions|ToFloat(Integer) (Variables|Default|GetUnitSkillSword)) (LocalVariables|GetNoClampLocal)))
            (Variables|HeroParams|SetUnitParExpSword _resultexp)
            (else
              (bind _resultexp_2 (CallFunction|HeroCalculateResultExp (Variables|HeroParams|GetUnitParExpSword) (LocalVariables|GetResultExpNotMainLocal) (Math|Conversions|ToFloat(Integer) (Variables|Default|GetUnitSkillSword)) (LocalVariables|GetNoClampLocal)))
              (Variables|HeroParams|SetUnitParExpSword _resultexp_2)))
          (bind _skillout (CallFunction|HeroCheckSkillsbyExp (Variables|Default|GetUnitSkillSword) (LocalVariables|GetNoClampLocal) (Variables|HeroParams|GetUnitParExpSword)))
          (Variables|Default|SetUnitSkillSword _skillout))
        (:NewEnumerator6
          (if (== (Variables|HeroParams|GetMainSkill) 3)
            (bind _resultexp_3 (CallFunction|HeroCalculateResultExp (Variables|HeroParams|GetUnitParExpMace) (LocalVariables|GetResultExpLocal) (Math|Conversions|ToFloat(Integer) (Variables|Default|GetUnitSkillMace)) (LocalVariables|GetNoClampLocal)))
            (Variables|HeroParams|SetUnitParExpMace _resultexp_3)
            (else
              (bind _resultexp_4 (CallFunction|HeroCalculateResultExp (Variables|HeroParams|GetUnitParExpMace) (LocalVariables|GetResultExpLocal) (Math|Conversions|ToFloat(Integer) (Variables|Default|GetUnitSkillMace)) (LocalVariables|GetNoClampLocal)))
              (Variables|HeroParams|SetUnitParExpMace _resultexp_4)))
          (bind _skillout_2 (CallFunction|HeroCheckSkillsbyExp (Variables|Default|GetUnitSkillMace) (LocalVariables|GetNoClampLocal) (Variables|HeroParams|GetUnitParExpMace)))
          (Variables|Default|SetUnitSkillMace _skillout_2))
        (:NewEnumerator7
          (if (== (Variables|HeroParams|GetMainSkill) 2)
            (bind _resultexp_5 (CallFunction|HeroCalculateResultExp (Variables|HeroParams|GetUnitParExpAxe) (LocalVariables|GetResultExpLocal) (Math|Conversions|ToFloat(Integer) (Variables|Default|GetUnitSkillAxe)) (LocalVariables|GetNoClampLocal)))
            (Variables|HeroParams|SetUnitParExpAxe _resultexp_5)
            (else
              (bind _resultexp_6 (CallFunction|HeroCalculateResultExp (Variables|HeroParams|GetUnitParExpAxe) (LocalVariables|GetResultExpLocal) (Math|Conversions|ToFloat(Integer) (Variables|Default|GetUnitSkillAxe)) (LocalVariables|GetNoClampLocal)))
              (Variables|HeroParams|SetUnitParExpAxe _resultexp_6)))
          (bind _skillout_3 (CallFunction|HeroCheckSkillsbyExp (Variables|Default|GetUnitSkillAxe) (LocalVariables|GetNoClampLocal) (Variables|HeroParams|GetUnitParExpAxe)))
          (Variables|Default|SetUnitSkillAxe _skillout_3))
        (:NewEnumerator8
          (if (== (Variables|HeroParams|GetMainSkill) 4)
            (bind _resultexp_7 (CallFunction|HeroCalculateResultExp (Variables|HeroParams|GetUnitParExpSpear) (LocalVariables|GetResultExpLocal) (Math|Conversions|ToFloat(Integer) (Variables|Default|GetUnitSkillSpear)) (LocalVariables|GetNoClampLocal)))
            (Variables|HeroParams|SetUnitParExpSpear _resultexp_7)
            (else
              (bind _resultexp_8 (CallFunction|HeroCalculateResultExp (Variables|HeroParams|GetUnitParExpSpear) (LocalVariables|GetResultExpLocal) (Math|Conversions|ToFloat(Integer) (Variables|Default|GetUnitSkillSpear)) (LocalVariables|GetNoClampLocal)))
              (Variables|HeroParams|SetUnitParExpSpear _resultexp_8)))
          (bind _skillout_4 (CallFunction|HeroCheckSkillsbyExp (Variables|Default|GetUnitSkillSpear) (LocalVariables|GetNoClampLocal) (Variables|HeroParams|GetUnitParExpSpear)))
          (Variables|Default|SetUnitSkillSpear _skillout_4))
        (:NewEnumerator9
          (if (== (Variables|HeroParams|GetMainSkill) 5)
            (bind _resultexp_9 (CallFunction|HeroCalculateResultExp (Variables|HeroParams|GetUnitParExpBow) (LocalVariables|GetResultExpLocal) (Math|Conversions|ToFloat(Integer) (Variables|Default|GetUnitSkillBow)) (LocalVariables|GetNoClampLocal)))
            (Variables|HeroParams|SetUnitParExpBow _resultexp_9)
            (else
              (bind _resultexp_10 (CallFunction|HeroCalculateResultExp (Variables|HeroParams|GetUnitParExpBow) (LocalVariables|GetResultExpLocal) (Math|Conversions|ToFloat(Integer) (Variables|Default|GetUnitSkillBow)) (LocalVariables|GetNoClampLocal)))
              (Variables|HeroParams|SetUnitParExpBow _resultexp_10)))
          (bind _skillout_5 (CallFunction|HeroCheckSkillsbyExp (Variables|Default|GetUnitSkillBow) (LocalVariables|GetNoClampLocal) (Variables|HeroParams|GetUnitParExpBow)))
          (Variables|Default|SetUnitSkillBow _skillout_5))
        (:NewEnumerator0
          (if _returnvalue
            (if (== (Variables|HeroParams|GetMainSkill) 1)
              (bind _resultexp_11 (CallFunction|HeroCalculateResultExp (Variables|HeroParams|GetUnitParExpFire) (LocalVariables|GetResultExpLocal) (Math|Conversions|ToFloat(Integer) (Variables|Default|GetUnitSkillFire)) (LocalVariables|GetNoClampLocal)))
              (Variables|HeroParams|SetUnitParExpFire _resultexp_11)
              (else
                (bind _resultexp_12 (CallFunction|HeroCalculateResultExp (Variables|HeroParams|GetUnitParExpFire) (LocalVariables|GetResultExpLocal) (Math|Conversions|ToFloat(Integer) (Variables|Default|GetUnitSkillFire)) (LocalVariables|GetNoClampLocal)))
                (Variables|HeroParams|SetUnitParExpFire _resultexp_12)))
            (bind _skillout_6 (CallFunction|HeroCheckSkillsbyExp (Variables|Default|GetUnitSkillFire) (LocalVariables|GetNoClampLocal) (Variables|HeroParams|GetUnitParExpFire)))
            (Variables|Default|SetUnitSkillFire _skillout_6)))
        (:NewEnumerator1
          (if _returnvalue
            (if (== (Variables|HeroParams|GetMainSkill) 2)
              (bind _resultexp_13 (CallFunction|HeroCalculateResultExp (Variables|HeroParams|GetUnitParExpWater) (LocalVariables|GetResultExpLocal) (Math|Conversions|ToFloat(Integer) (Variables|Default|GetUnitSkillWater)) (LocalVariables|GetNoClampLocal)))
              (Variables|HeroParams|SetUnitParExpWater _resultexp_13)
              (else
                (bind _resultexp_14 (CallFunction|HeroCalculateResultExp (Variables|HeroParams|GetUnitParExpWater) (LocalVariables|GetResultExpLocal) (Math|Conversions|ToFloat(Integer) (Variables|Default|GetUnitSkillWater)) (LocalVariables|GetNoClampLocal)))
                (Variables|HeroParams|SetUnitParExpWater _resultexp_14)))
            (bind _skillout_7 (CallFunction|HeroCheckSkillsbyExp (Variables|Default|GetUnitSkillWater) (LocalVariables|GetNoClampLocal) (Variables|HeroParams|GetUnitParExpWater)))
            (Variables|Default|SetUnitSkillWater _skillout_7)))
        (:NewEnumerator2
          (if _returnvalue
            (if (== (Variables|HeroParams|GetMainSkill) 3)
              (bind _resultexp_15 (CallFunction|HeroCalculateResultExp (Variables|HeroParams|GetUnitParExpAir) (LocalVariables|GetResultExpLocal) (Math|Conversions|ToFloat(Integer) (Variables|Default|GetUnitSkillAir)) (LocalVariables|GetNoClampLocal)))
              (Variables|HeroParams|SetUnitParExpAir _resultexp_15)
              (else
                (bind _resultexp_16 (CallFunction|HeroCalculateResultExp (Variables|HeroParams|GetUnitParExpAir) (LocalVariables|GetResultExpLocal) (Math|Conversions|ToFloat(Integer) (Variables|Default|GetUnitSkillAir)) (LocalVariables|GetNoClampLocal)))
                (Variables|HeroParams|SetUnitParExpAir _resultexp_16)))
            (bind _skillout_8 (CallFunction|HeroCheckSkillsbyExp (Variables|Default|GetUnitSkillAir) (LocalVariables|GetNoClampLocal) (Variables|HeroParams|GetUnitParExpAir)))
            (Variables|Default|SetUnitSkillAir _skillout_8)))
        (:NewEnumerator3
          (if _returnvalue
            (if (== (Variables|HeroParams|GetMainSkill) 4)
              (bind _resultexp_17 (CallFunction|HeroCalculateResultExp (Variables|HeroParams|GetUnitParExpEarth) (LocalVariables|GetResultExpLocal) (Math|Conversions|ToFloat(Integer) (Variables|Default|GetUnitSkillEarth)) (LocalVariables|GetNoClampLocal)))
              (Variables|HeroParams|SetUnitParExpEarth _resultexp_17)
              (else
                (bind _resultexp_18 (CallFunction|HeroCalculateResultExp (Variables|HeroParams|GetUnitParExpEarth) (LocalVariables|GetResultExpLocal) (Math|Conversions|ToFloat(Integer) (Variables|Default|GetUnitSkillEarth)) (LocalVariables|GetNoClampLocal)))
                (Variables|HeroParams|SetUnitParExpEarth _resultexp_18)))
            (bind _skillout_9 (CallFunction|HeroCheckSkillsbyExp (Variables|Default|GetUnitSkillEarth) (LocalVariables|GetNoClampLocal) (Variables|HeroParams|GetUnitParExpEarth)))
            (Variables|Default|SetUnitSkillEarth _skillout_9)))
        (:NewEnumerator4
          (if _returnvalue
            (if (== (Variables|HeroParams|GetMainSkill) 5)
              (bind _resultexp_19 (CallFunction|HeroCalculateResultExp (Variables|HeroParams|GetUnitParExpAstral) (LocalVariables|GetResultExpLocal) (Math|Conversions|ToFloat(Integer) (Variables|Default|GetUnitSkillAstral)) (LocalVariables|GetNoClampLocal)))
              (Variables|HeroParams|SetUnitParExpAstral _resultexp_19)
              (else
                (bind _resultexp_20 (CallFunction|HeroCalculateResultExp (Variables|HeroParams|GetUnitParExpAstral) (LocalVariables|GetResultExpLocal) (Math|Conversions|ToFloat(Integer) (Variables|Default|GetUnitSkillAstral)) (LocalVariables|GetNoClampLocal)))
                (Variables|HeroParams|SetUnitParExpAstral _resultexp_20)))
            (bind _skillout_10 (CallFunction|HeroCheckSkillsbyExp (Variables|Default|GetUnitSkillAstral) (LocalVariables|GetNoClampLocal) (Variables|HeroParams|GetUnitParExpAstral)))
            (Variables|Default|SetUnitSkillAstral _skillout_10)))))
    (:then_1
      (Variables|HeroParams|SetUnitParExperience (Math|Float|Truncate (+ (Variables|HeroParams|GetUnitParExpSword) (Variables|HeroParams|GetUnitParExpMace) (Variables|HeroParams|GetUnitParExpAxe) (Variables|HeroParams|GetUnitParExpSpear) (Variables|HeroParams|GetUnitParExpBow) (Variables|HeroParams|GetUnitParExpFire) (Variables|HeroParams|GetUnitParExpWater) (Variables|HeroParams|GetUnitParExpAir) (Variables|HeroParams|GetUnitParExpEarth) (Variables|HeroParams|GetUnitParExpAstral)))))))

(fn HeroCheckSkillsbyExp
  (params (UnitSkill :type Integer) (Silent :type Boolean) (UnitSkillExp :type Float%20%28single-precision%29))
  (LocalVariables|SetSkillLocal UnitSkill)
  (Utilities|FlowControl|ForLoopwithBreak 0 99 :!label _label
    (:LoopBody
      (bind _out (CallFunction|HeroA3Skill2Exp (Math|Conversions|ToFloat(Integer) (LocalVariables|GetSkillLocal))))
      (if (> UnitSkillExp _out)
        (Math|Integer|IncrementInt (LocalVariables|GetSkillLocal))
        (else
          (goto _label Break))))
    (:Completed
      (if (not Silent)
        _
        (else
          _))
      (return (LocalVariables|GetSkillLocal)))))