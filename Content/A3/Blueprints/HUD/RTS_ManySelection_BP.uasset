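; RTS HUD that handles drag-box selection of RTS_UnitMaster_BP units.
; Input events track the mouse rectangle, starting only outside map, inventory and right panel and when no characters are selected.
; DrawHUD draws the marquee and highlights fully enclosed units via UnitFocused, using a touched-units list to clear stale highlights.
; Release passes enclosed units to the player controller's AISelectF, keeping focus when exactly one is selected.
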(event Custom|DrawMarque
  (bind _clickedlocation (Variables|Default|GetClickedLocation))
  (bind _holdinglocation (Variables|Default|GetHoldingLocation))
  (bind _clickedlocation_2 (Variables|Default|GetClickedLocation))
  (bind _holdinglocation_2 (Variables|Default|GetHoldingLocation))
  (bind _clickedlocation_3 (Variables|Default|GetClickedLocation))
  (bind _clickedlocation_4 (Variables|Default|GetClickedLocation))
  (bind _holdinglocation_3 (Variables|Default|GetHoldingLocation))
  (bind _returnvalue (- _holdinglocation_3 _clickedlocation_4))
  (bind (_x _y) (Math|Vector2D|BreakVector2D _returnvalue))
  (HUD|DrawRect "(R=0.479167,G=0.442577,B=0.034687,A=0.300000)" (.x _clickedlocation) (.y _clickedlocation) _x _y)
  (Class|HUD|DrawLine (.x _clickedlocation_2) (.y _clickedlocation_2) (.x _clickedlocation_2) (.y (Variables|Default|GetHoldingLocation)) "(R=0.630208,G=0.485577,B=0.032823,A=1.000000)" 1.0)
  (Class|HUD|DrawLine (.x _holdinglocation_2) (.y (Variables|Default|GetClickedLocation)) (.x _holdinglocation_2) (.y _holdinglocation_2) "(R=0.630208,G=0.485577,B=0.032823,A=1.000000)" 1.0)
  (Class|HUD|DrawLine (.x _clickedlocation_3) (.y _clickedlocation_3) (.x (Variables|Default|GetHoldingLocation)) (.y _clickedlocation_3) "(R=0.630208,G=0.485577,B=0.032823,A=1.000000)" 1.0)
  (Class|HUD|DrawLine (.x (Variables|Default|GetClickedLocation)) (.y _holdinglocation) (.x _holdinglocation) (.y _holdinglocation) "(R=0.630208,G=0.485577,B=0.032823,A=1.000000)" 1.0))

(event EventBeginPlay
  (bind _asrts_player_controller_bp (Utilities|Casting|CastToRTS_PlayerController_BP (Game|GetPlayerController 0)))
  (Variables|References|SetPlaye%20ControllerRef _asrts_player_controller_bp))

(event EventDrawHUD
  (params (SizeX :type Integer) (SizeY :type Integer))
  (bind _clickedlocation (Variables|Default|GetClickedLocation))
  (bind _holdinglocation (Variables|Default|GetHoldingLocation))
  (bind _outactors (Class|HUD|GetActorsinSelectionRectangle "/Game/A3/Blueprints/Units/MastersBP/RTS_UnitMaster_BP.RTS_UnitMaster_BP_C" _clickedlocation _holdinglocation false true))
  (if (Variables|Default|GetIsDrawing?)
    (CallFunction|DrawMarque)
    (CallFunction|MakePoints)
    (for _array_element _outactors
      (Utilities|Array|AddUnique (Variables|Default|GetUnitsWasInSelectionArea) _array_element))
    (Variables|Default|SetUnitsInSelectionArea _outactors)
    (Utilities|FlowControl|Sequence
      (:then_0
        (for _array_element_2 (Variables|Default|GetUnitsWasInSelectionArea)
          (bind _outunit (CallFunction|GetUnitMaster _array_element_2))
          (if (Variables|/Game/A3/Blueprints/Units/MastersBP/RTS_UnitMaster_BP.RTS_UnitMaster_BP_C|GetUnitFocused _outunit)
            (Variables|/Game/A3/Blueprints/Units/MastersBP/RTS_UnitMaster_BP.RTS_UnitMaster_BP_C|SetUnitFocused _outunit false))))
      (:then_1
        (for _array_element_3 (Variables|Default|GetUnitsInSelectionArea)
          (bind _outunit_2 (CallFunction|GetUnitMaster _array_element_3))
          (if (not (Variables|/Game/A3/Blueprints/Units/MastersBP/RTS_UnitMaster_BP.RTS_UnitMaster_BP_C|GetUnitFocused _outunit_2))
            (Variables|/Game/A3/Blueprints/Units/MastersBP/RTS_UnitMaster_BP.RTS_UnitMaster_BP_C|SetUnitFocused _outunit_2 true)))))))

(event EventOnInputStartF
  (bind _playe_controllerref (Variables|References|GetPlaye%20ControllerRef))
  (bind _playe_controllerref_2 (Variables|References|GetPlaye%20ControllerRef))
  (bind (_locationx _locationy) (Game|Player|GetMousePosition _playe_controllerref_2))
  (bind _returnvalue (Math|Vector2D|MakeVector2D _locationx _locationy))
  (if (not (Math|Boolean|ORBoolean (Variables|/Game/A3/Blueprints/Player/RTS_PlayerController_BP.RTS_PlayerController_BP_C|GetAtMap? _playe_controllerref) (Variables|/Game/A3/Blueprints/Player/RTS_PlayerController_BP.RTS_PlayerController_BP_C|GetAtInventory? _playe_controllerref) (Variables|/Game/A3/Blueprints/Player/RTS_PlayerController_BP.RTS_PlayerController_BP_C|GetAtRightPanel? _playe_controllerref)))
    (if (not (>= (Utilities|Array|LastIndex (Variables|/Game/A3/Blueprints/Player/RTS_PlayerController_BP.RTS_PlayerController_BP_C|GetSelected%20Characters _playe_controllerref)) 0))
      (Variables|Default|SetClickedLocation _returnvalue)
      (Variables|Default|SetHoldingLocation _returnvalue)
      (Variables|Default|SetIsDrawing? true))))

(event EventOnInputHoldF
  (bind _playe_controllerref (Variables|References|GetPlaye%20ControllerRef))
  (bind (_locationx _locationy) (Game|Player|GetMousePosition _playe_controllerref))
  (Variables|Default|SetHoldingLocation (Math|Vector2D|MakeVector2D _locationx _locationy)))

(event EventOnInputReleaseF
  (params (HoldTime :type Float%20%28single-precision%29))
  (bind _unitsinselectionarea (Variables|Default|GetUnitsInSelectionArea))
  (bind _playe_controllerref (Variables|References|GetPlaye%20ControllerRef))
  (Variables|Default|SetIsDrawing? false)
  (for _array_element _unitsinselectionarea
    (bind _outunit (CallFunction|GetUnitMaster _array_element))
    (Default|AISelectF (Variables|References|GetPlaye%20ControllerRef) _outunit)
    (Variables|/Game/A3/Blueprints/Units/MastersBP/RTS_UnitMaster_BP.RTS_UnitMaster_BP_C|SetUnitFocused _outunit false)
    (if (== (Utilities|Array|Length (Variables|/Game/A3/Blueprints/Player/RTS_PlayerController_BP.RTS_PlayerController_BP_C|GetSelected%20Characters _playe_controllerref)) 1)
      (Variables|/Game/A3/Blueprints/Units/MastersBP/RTS_UnitMaster_BP.RTS_UnitMaster_BP_C|SetUnitFocused _outunit true)
      (Default|TraceTargetIsNotUnit _playe_controllerref)))
  (Utilities|Array|Clear _unitsinselectionarea)
  (Utilities|Array|Clear (Variables|Default|GetUnitsWasInSelectionArea)))

(fn ConstructionScript)

(fn GetUnitMaster
  (params (Unit :type Actor%20Object%20Reference))
  (if (Utilities|ClassIsChildOf (Utilities|GetClass Unit) "/Game/A3/Blueprints/Units/MastersBP/RTS_UnitMaster_BP.RTS_UnitMaster_BP_C")
    (bind _asrts_unit_master_bp (Utilities|Casting|CastToRTS_UnitMaster_BP Unit))
    (return _asrts_unit_master_bp)))

(fn MakePoints
  (bind _clickedlocation (Variables|Default|GetClickedLocation))
  (bind _holdinglocation (Variables|Default|GetHoldingLocation))
  (bind _clickedlocation_2 (Variables|Default|GetClickedLocation))
  (bind _holdinglocation_2 (Variables|Default|GetHoldingLocation))
  (if (Math|Vector|Equal(Vector) _clickedlocation _holdinglocation 0.0001)
    (Variables|Default|SetSubPointStart _clickedlocation :!label _label)
    (Variables|Default|SetSubPointEnd _holdinglocation)
    (elif (> (.x _clickedlocation_2) (.x _holdinglocation_2))
      (Variables|Default|SetSubPointStart (Math|Vector2D|MakeVector2D (- (.x _clickedlocation_2) (Variables|Default|GetAddToBox)) (.y _clickedlocation_2)))
      (Variables|Default|SetSubPointEnd (Math|Vector2D|MakeVector2D (+ (.x _holdinglocation_2) (Variables|Default|GetAddToBox)) (.y _clickedlocation_2)))
      (else
        (goto _label))))
  (return))