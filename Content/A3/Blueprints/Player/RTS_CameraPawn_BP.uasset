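; RTS camera pawn that can keep itself at ground height.
; SetZposition line-traces vertically on Visibility at the pawn's current XY, ignoring RTS unit actors, and takes the hit's Z.
; On a hit, it moves the pawn to that height at either the supplied XY or the Sphere component's XY.
; BeginPlay sets a fixed rotation and prints a leftover "Died" message, while Tick is empty.
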(event EventTick
  (params (DeltaSeconds :type Float%20%28single-precision%29)))

(event EventBeginPlay
  (Transformation|SetActorRotation "20.000000,0.000000, 0" true)
  (Development|PrintString "Died"))

(fn ConstructionScript)

(fn SetZposition
  (params (SetLocation :type Boolean) (LocX :type Float%20%28single-precision%29) (LoxY :type Float%20%28single-precision%29))
  (bind _returnvalue (Transformation|GetActorLocation))
  (bind _sphere (Variables|Default|GetSphere))
  (bind _returnvalue_2 (Transformation|GetWorldLocation _sphere))
  (bind _asrts_unit_master_bp (Utilities|Casting|CastToRTS_UnitMaster_BPClass "/Game/A3/Blueprints/Units/MastersBP/RTS_UnitMaster_BP.RTS_UnitMaster_BP_C"))
  (bind _outactors (Actor|GetAllActorsOfClass _asrts_unit_master_bp))
  (bind (_outhit _returnvalue_3) (Collision|LineTraceByChannel (Math|Vector|MakeVector (.x _returnvalue) (.y _returnvalue) 2e+04) (Math|Vector|MakeVector (.x _returnvalue) (.y _returnvalue) -2e+04) "TraceTypeQuery1" false _outactors "None"))
  (if _returnvalue_3
    (if SetLocation
      (Transformation|SetActorLocation (Math|Vector|MakeVector LocX LoxY (.Z (Math|Vector|BreakVector (.Location (Collision|BreakHitResult _outhit))))) false false)
      (else
        (Transformation|SetActorLocation (Math|Vector|MakeVector (.x _returnvalue_2) (.y _returnvalue_2) (.Z (Math|Vector|BreakVector (.Location (Collision|BreakHitResult _outhit))))) false false)))))