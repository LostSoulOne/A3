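; Item bag pickup actor that holds items and hands them to an RTS unit on overlap.
; Construction gives the mesh a random yaw and wraps each ItemsContain entry in a UData object stored in ContainingItems.
; Overlap by a unit of UnitClass 5 transfers all items to its inventory, destroys the bag and refreshes the player controller's inventory.
; Helpers for adding item objects and zero-filling magic parameters are uncalled here.
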(event OnComponentBeginOverlap(StaticMesh)
  (params (OverlappedComponent :type Primitive%20Component%20Object%20Reference) (OtherActor :type Actor%20Object%20Reference) (OtherComp :type Primitive%20Component%20Object%20Reference) (OtherBodyIndex :type Integer) (bFromSweep :type Boolean) (SweepResult :type Hit%20Result%20Structure%20%28by%20ref%29))
  ;[1 1 1] Поднятие мешка
  (CallFunction|UnitTakeItem (stale Collision|EventActorBeginOverlap OtherActor)))

(event EventBeginPlay)

(event Collision|EventActorBeginOverlap
  (params (OtherActor :type Actor%20Object%20Reference))
  ;[1 1 1] Поднятие мешка
  (CallFunction|UnitTakeItem OtherActor))

(fn ConstructionScript
  (Transformation|SetRelativeRotation (Variables|Default|GetStaticMesh) (Math|Rotator|MakeRotator 0.0 0.0 (* (Math|Random|RandomFloat) 3.6e+02)) false false)
  (for _array_element (Variables|Default|GetItemsContain)
    (CallFunction|AddItemDatatoBagasObj _array_element)))

(fn AddItemDatatoBagasObj
  (params (NewData :type Item%20Info%20Data%20Structure))
  (bind _returnvalue (Game|ConstructObjectfromClass "/Game/A3/Blueprints/Inventory/UData.UData_C" self))
  (Utilities|Array|Add (Variables|Items|GetContainingItems) _returnvalue)
  (Variables|/Game/A3/Blueprints/Inventory/UData.UData_C|SetData _returnvalue NewData))

(fn AddItemtoBag
  (params (ItemObject :type U%20Data%20Object%20Reference%20%28by%20ref%29))
  (bind _containingitems (Variables|Items|GetContainingItems))
  (bind _returnvalue (Utilities|Array|FindItem _containingitems ItemObject))
  (bind _output (Utilities|Array|Get(acopy) _containingitems _returnvalue))
  (bind _data (Variables|/Game/A3/Blueprints/Inventory/UData.UData_C|GetData _output))
  ;[1 1 1] Это всё неправильная хуйня
  (if (== _returnvalue -1)
    (Utilities|Array|Add _containingitems ItemObject)
    (else
      (Utilities|Struct|SetmembersinItemInfoData _data (+ (.Count (Utilities|Struct|BreakItemInfoData (Variables|/Game/A3/Blueprints/Inventory/UData.UData_C|GetData ItemObject))) (.Count (Utilities|Struct|BreakItemInfoData _data)))))))

(fn AddMagicParameters
  (bind _outrownames (DataTable|GetDataTableRowNames "/Game/A3/DataFiles/dBaseItemParameters.dBaseItemParameters"))
  (for _array_element _outrownames
    (Utilities|Map|Add (Variables|Default|GetMagicParameters) (Utilities|String|ToString(Name) _array_element) 0)))

(fn UnitTakeItem
  (params (Actor :type Actor%20Object%20Reference))
  (bind _asrts_unit_master_bp (Utilities|Casting|CastToRTS_UnitMaster_BP Actor)
    (:then
      (if (== (Variables|/Game/A3/Blueprints/Units/MastersBP/RTS_UnitMaster_BP.RTS_UnitMaster_BP_C|GetUnitClass _asrts_unit_master_bp) 5)
        (for _array_element (Variables|Items|GetContainingItems)
          (Default|AddItemtoInventory _asrts_unit_master_bp _array_element))
        (Actor|DestroyActor)
        (bind _asrts_player_controller_bp (Utilities|Casting|CastToRTS_PlayerController_BP (Pawn|GetController (Game|Player|GetPlayerPawn 0)))
          (:then
            (Default|UpdateInventoryItemsF _asrts_player_controller_bp))
          (:CastFailed
            _))))
    (:CastFailed
      _))
  (return))