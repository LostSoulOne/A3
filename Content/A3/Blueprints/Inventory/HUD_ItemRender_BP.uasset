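; Inventory HUD actor that presents an item mesh and spins it while the IsCaptured flag is set.
; BeginPlay applies the mesh's X offset and uniform scale.
; Tick adds a per-frame angle step to the Sphere component's roll, wrapped at 360, with fixed pitch and yaw offsets.
; RotationStart ramps that step up, and RotationEnding winds it down as the turn nears completion once capture ends, independent of frame time.
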(event EventBeginPlay
  (CallFunction|UpdatePositionXOffset)
  (CallFunction|UpdateScale))

(event EventTick
  (params (DeltaSeconds :type Float%20%28single-precision%29))
  (Variables|Default|SetTimeDelta DeltaSeconds)
  (Utilities|FlowControl|Sequence
    (:then_0
      (if (> (Variables|Default|GetRotationAddtionalAngle) 0.0)
        (Variables|Default|SetCurrentRotationX (- (+ (Variables|Default|GetCurrentRotationX) (Variables|Default|GetRotationAddtionalAngle)) (Math|Conversions|ToFloat(Integer) (* (.ReturnValue (Math|Float|Division(WholeandRemainder) (+ (Variables|Default|GetCurrentRotationX) (Variables|Default|GetRotationAddtionalAngle)) 3.6e+02)) 360))))
        (if (!= (Variables|Default|GetCurrentRotationX) 0.0)
          (CallFunction|SetItemRotation))))
    (:then_1
      (if (Variables|Default|GetIsCaptured?)
        (Variables|Default|SetLetsSpeedUp! true)
        (else
          (Variables|Default|SetLetsSlowDown! true))))
    (:then_2
      (if (Variables|Default|GetLetsSpeedUp!)
        (Utilities|RotationStart)))
    (:then_3
      (if (and (Variables|Default|GetLetsSlowDown!) (not (Variables|Default|GetIsCaptured?)))
        (Utilities|RotationEnding)))))

(fn ConstructionScript)

(fn RotateItem
  (params (DeltaTime :type Float%20%28single-precision%29) (TargetAngle :type Float%20%28single-precision%29) (InterpSpeed :type Float%20%28single-precision%29))
  (Variables|Default|SetRotationAddtionalAngle 3e+01))

(fn UpdatePositionXOffset
  (Transformation|SetRelativeLocation (Variables|Default|GetStaticMesh) (Math|Vector|MakeVector (Variables|Default|GetOffsetPositionX) 0.0 0.0) false false))

(fn UpdateScale
  (bind _staticmesh (Variables|Default|GetStaticMesh))
  (Transformation|SetRelativeTransform _staticmesh (Math|Transform|MakeTransform (Variables|/Script/Engine.SceneComponent|GetRelativeLocation _staticmesh) (Variables|/Script/Engine.SceneComponent|GetRelativeRotation _staticmesh) (Math|Conversions|ToVector(Float) (Variables|Default|GetCurrentScale))) false false))

(fn SetItemRotation
  (Transformation|SetRelativeRotation (Variables|Default|GetSphere) (Math|Rotator|MakeRotator (Variables|Default|GetCurrentRotationX) (Variables|Default|GetOffsetRotationY) (Variables|Default|GetOffsetRotationZ)) false false))